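; Enemy AI character that can be knocked back and temporarily stunned through character interface events.
; It caches its AI controller's brain component at BeginPlay, then stuns by stopping that logic and restarting it after a delay.
; Knockback passes the given force to LaunchCharacter, adding to current velocity.
; A debug event prints a point just behind the enemy, and unconnected movement test nodes remain.
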(event `Debug_TurnAround`
  (bind _returnvalue (`self.GetActorForwardVector`))
  ;[1 1 1] GetTurnaroundLocation
  (`KismetSystemLibrary.PrintString` (`KismetStringLibrary.Concat_StrStr` (`KismetStringLibrary.Conv_VectorToString` _returnvalue) (`KismetStringLibrary.Conv_VectorToString` (+ (`self.K2_GetActorLocation`) (* _returnvalue -2.0))))))

(event `self.ReceiveBeginPlay`
  (set `self.Brain Component` (`AIController.BrainComponent` (`AIBlueprintHelperLibrary.GetAIController` self))))

(event `/Game/Blueprint/Player/Character_INT.ApplyKnockback`
  (params (Force :type "Vector Structure"))
  ;[1 1 1] Character INT
  (`self.LaunchCharacter` Force))

(event `/Game/Blueprint/Player/Character_INT.StunCharacter`
  (params (Duration :type "Float (single-precision)"))
  (bind _brain_component (`self.Brain Component`))
  ;[1 1 1] Character INT
  (`BrainComponent.StopLogic` _brain_component "")
  (`KismetSystemLibrary.Delay` Duration)
  (`BrainComponent.StartLogic` _brain_component))

(fn `UserConstructionScript`)