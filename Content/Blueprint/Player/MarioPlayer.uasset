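; Mario player Blueprint that gives the player a melee attack on left mouse click.
; A sphere overlap at AttackPositionComponent gathers nearby Pawns, excluding itself.
; Each hit actor implementing Character_INT receives interface messages for a horizontal knockback away from the player and a timed stun.
; The attack also prints each target's offset, and the other events and construction script are empty.
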(event `Key|LeftMouseButton`
  (params (Key :type "Key Structure"))
  (:`Pressed`
    (bind _outactors (`KismetSystemLibrary.SphereOverlapActors` (`SceneComponent.K2_GetComponentLocation` (`self.AttackPositionComponent`)) 50.0 (`|MakeArray` "ObjectTypeQuery3" :!type "EObjectTypeQuery Enum") null (`|MakeArray` self :!type "Actor Object Reference")))
    (for _array_element _outactors
      (if (`KismetSystemLibrary.DoesImplementInterface` _array_element "/Game/Blueprint/Player/Character_INT.Character_INT_C")
        (bind _returnvalue (- (`self.K2_GetActorLocation` _array_element) (`self.K2_GetActorLocation`)))
        (message `/Game/Blueprint/Player/Character_INT.ApplyKnockback` _array_element (* (`KismetMathLibrary.Vector_Normal2D` _returnvalue) 2000.0))
        (`KismetSystemLibrary.PrintString` (`KismetStringLibrary.Conv_VectorToString` _returnvalue))
        (message `/Game/Blueprint/Player/Character_INT.StunCharacter` _array_element 2.0)))))

(fn `UserConstructionScript`)